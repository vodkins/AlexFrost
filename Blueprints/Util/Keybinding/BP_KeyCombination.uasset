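; Keybinding object for one key combination, built from digital, analog-axis or mouse-delta key input objects and polled through a player controller.
; Its state multiplies key axis values and derives active, just-pressed and just-released from per-key counts.
; Overlaps with other combinations are classified for menu display, and selected types block input, synthesizing press and release edges.
; It also saves, loads with default fallback, and generates shortened display names.
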(fn InitKeyCombination
  (params (Name :type String) (Can't%20Be%20None :type Boolean) (Key%20Combination :type Array%20of%20S%20Key%20Input%20Structures))
  (Variables|Default|SetName Name)
  (Variables|Default|SetCan't%20Be%20None Can't%20Be%20None)
  (bind _output_get (Variables|Default|SetDefault%20Combination Key%20Combination))
  (for _array_element _output_get
    (CallFunction|AddKeyInput _array_element))
  (return self))

(fn KeyCombinationCurrentState
  (params (Player%20Controller :type Player%20Controller%20Object%20Reference) (Ignore%20Conflicts :type Boolean))
  (bind _keys_currently_pressed (LocalVariables|GetKeys%20Currently%20Pressed))
  (bind _keys_pressed_from_last_frame (LocalVariables|GetKeys%20Pressed%20From%20Last%20Frame))
  (bind _keys_released_from_last_frame (LocalVariables|GetKeys%20Released%20From%20Last%20Frame))
  (bind (_is_active _just_pressed _just_released) (|GetCombinationState _keys_pressed_from_last_frame _keys_currently_pressed _keys_released_from_last_frame))
  (if (> (Utilities|Array|Length (Variables|Default|GetKey%20Inputs)) 0)
    (LocalVariables|SetCombination%20Value 1.0)
    (for _array_element (Variables|Default|GetKey%20Inputs)
      (bind (_axis_value _down _just_pressed_2 _just_released_2) (Default|KeyInputCurrentState _array_element Player%20Controller))
      (LocalVariables|SetCombination%20Value (* _axis_value (LocalVariables|GetCombination%20Value)))
      (Utilities|IncrementIntifTrue (LocalVariables|GetKeys%20Currently%20Pressed) _down
        (:%20%20
          (Utilities|IncrementIntifTrue (LocalVariables|GetKeys%20Pressed%20From%20Last%20Frame) _just_pressed_2
            (:%20%20
              (Utilities|IncrementIntifTrue (LocalVariables|GetKeys%20Released%20From%20Last%20Frame) _just_released_2))))))
    (if Ignore%20Conflicts ; Check if we want to consider \nconflicting combinations
      (return (LocalVariables|GetCombination%20Value) _is_active _just_pressed _just_released)
      (else
        (bind (_is_active_2 _just_pressed_3 _just_released_3) (Conflict|EvaluateBlockingCombinations Player%20Controller))
        (if _is_active_2
          (return 0.0 false false (Math|Boolean|ANDBoolean _just_pressed_3 _is_active (not _just_pressed))) ; Input Is blocked\nSee if it was enabled last frame,\nbut blocked this frame\nThen "Just Released" is true due to conflict.
          (else
            (return (LocalVariables|GetCombination%20Value) _is_active (or (and _just_released_3 _is_active) _just_pressed) _just_released) ; See if it was blocked last frame,\nbut not this frame. Then\n"Just Pressed" is true
          ))))
    (else
      (return 0.0 false false false) ; No keybindings exists
    )))

(fn SaveKeyCombination
  (params (Game%20Settings :type BP%20Game%20Settings%20Object%20Reference) (KeySave :type S%20Key%20Action%20Save%20Structure%20%28by%20ref%29))
  (bind _returnvalue (|Copy KeySave))
  (for _array_element (Variables|Default|GetKey%20Inputs)
    (Default|SaveKeyInput _array_element Game%20Settings _returnvalue))
  (if (== (Utilities|Array|Length (Variables|Default|GetKey%20Inputs)) 0)
    (bind _structout (Utilities|Struct|SetmembersinSKeyActionSave _returnvalue "AnyKey" false true))
    (Default|StoreKeyInput Game%20Settings _structout) ; Store empty combination so system\nknows it is intended to be empty
  ))

(fn LoadKeyCombination
  (params (Game%20Settings :type BP%20Game%20Settings%20Object%20Reference) (Action%20Name :type String) (Category :type String) (Name :type String) (Primary :type Boolean))
  (Utilities|Array|Clear (LocalVariables|GetLoaded%20Combination))
  (for _array_element (Default|GetSavedKeyInputs Game%20Settings) ; Search for matching mapping in game settings
    (if (Math|Boolean|ANDBoolean (Utilities|Enum|Equal(Enum) (.actionname _array_element) Action%20Name) (Utilities|Enum|Equal(Enum) (.category _array_element) Category) (Utilities|Enum|Equal(Enum) (.name _array_element) Name) (Math|Boolean|Equal(Boolean) (.primary _array_element) Primary)) ; Match found in gamesettings
      (if (.emptycombination _array_element)
        (LocalVariables|SetEmpty%20Combination true) ; Mapping is intentionally left empty,\nwe will remove default keys.
        (else
          (Utilities|Array|Add (LocalVariables|GetLoaded%20Combination) (Utilities|Struct|MakeSKeyInput (.keyinput _array_element) (.negativeaxis _array_element)))))))
  (if (== (Utilities|Array|Length (LocalVariables|GetLoaded%20Combination)) 0)
    (if (LocalVariables|GetEmpty%20Combination)
      (CallFunction|ReplaceKeyCombination (LocalVariables|GetLoaded%20Combination) :!label _label))
    (else
      (goto _label)))
  (return))

(fn ReplaceKeyCombination
  (params (Key%20Combination :type Array%20of%20S%20Key%20Input%20Structures))
  (bind _output_get (LocalVariables|SetNew%20combination Key%20Combination))
  (bind _result (CallFunction|EqualAllKeys _output_get))
  (if (not _result) ; Do nothing if keys are\nequal to existing ones
    (if (and (== (Utilities|Array|Length _output_get) 0) (Variables|Default|GetCan't%20Be%20None)) ; Return to default if binding\nis not allowed to be none
      (LocalVariables|SetNew%20combination (Variables|Default|GetDefault%20Combination)))
    (Utilities|Array|Clear (Variables|Default|GetKey%20Inputs))
    (for _array_element (LocalVariables|GetNew%20combination)
      (CallFunction|AddKeyInput _array_element))
    (Default|CallCombinationUpdated self)))

(fn DetectConflict
  (params (Input%20Combination :type BP%20Key%20Combination%20Object%20Reference))
  (bind _key_inputs (Variables|BP_KeyCombination_C|GetKey%20Inputs Input%20Combination))
  (bind _key_inputs_2 (Variables|Default|GetKey%20Inputs))
  (bind _returnvalue (Utilities|Array|Length _key_inputs))
  (bind _returnvalue_2 (Utilities|Array|Length _key_inputs_2))
  (for _array_element _key_inputs ; For every key in input array
    (for _array_element_2 (Variables|Default|GetKey%20Inputs) ; See if there is a match with\nkeys in current combination
      (if (and (Math|Boolean|Equal(Boolean) (Variables|/Game/QualityMenu/Blueprints/Util/Keybinding/BP_KeyInput.BP_KeyInput_C|GetAnalog%20Use%20Negative%20Axis _array_element_2) (Variables|/Game/QualityMenu/Blueprints/Util/Keybinding/BP_KeyInput.BP_KeyInput_C|GetAnalog%20Use%20Negative%20Axis _array_element)) (== (Variables|/Game/QualityMenu/Blueprints/Util/Keybinding/BP_KeyInput.BP_KeyInput_C|GetKey%20Input _array_element) (Variables|/Game/QualityMenu/Blueprints/Util/Keybinding/BP_KeyInput.BP_KeyInput_C|GetKey%20Input _array_element_2)))
        (Math|Integer|IncrementInt (LocalVariables|GetMatching%20Inputs)
          (:%20%20
            (Utilities|IncrementIntifTrue (LocalVariables|GetMatching%20Modifier%20Inputs) (Class|KismetInputLibrary|KeyIsModifierKey (Variables|/Game/QualityMenu/Blueprints/Util/Keybinding/BP_KeyInput.BP_KeyInput_C|GetKey%20Input _array_element_2))))))))
  (if (== (LocalVariables|GetMatching%20Inputs) 0)
    (return "NewEnumerator5") ; No keys are conflicting
    (else
      (Utilities|FlowControl|Sequence
        (:then_0
          (Math|Integer|CompareInt _returnvalue _returnvalue_2
            (:>
              ;[1 1 1] Check if input is a Superset and contains all inputs of this keycombination
              (if (== _returnvalue_2 (LocalVariables|GetMatching%20Inputs))
                (LocalVariables|SetConflict "NewEnumerator3")
                (else
                  (LocalVariables|SetConflict "NewEnumerator1"))))
            (:==
              ;[1 1 1] Check if input is equal and share all its keys with this keycombination
              (if (== _returnvalue_2 (LocalVariables|GetMatching%20Inputs))
                (LocalVariables|SetConflict "NewEnumerator0")
                (else
                  (LocalVariables|SetConflict "NewEnumerator1"))))
            (:<
              ;[1 1 1] Check if input is is a subset and this combination contains all input keys
              (if (== _returnvalue (LocalVariables|GetMatching%20Inputs))
                (LocalVariables|SetConflict "NewEnumerator2")
                (else
                  (LocalVariables|SetConflict "NewEnumerator1"))))))
        (:then_1
          (if (and (Utilities|Enum|Equal(Enum) (LocalVariables|GetConflict) "NewEnumerator1") (== (LocalVariables|GetMatching%20Inputs) (LocalVariables|GetMatching%20Modifier%20Inputs))) ; See if all overlapping keys are\nmodifier keys. (Players are\nusually not bothered by shared\nmodifiers in keybindings)
            (LocalVariables|SetConflict "NewEnumerator4"))
          (return (LocalVariables|GetConflict)))))))

(fn AddConflictingCombination
  (params (Conflicted%20Combination :type BP%20Key%20Combination%20Object%20Reference) (Conflicted%20 :type EKeyConflict%20Enum))
  (Utilities|FlowControl|Sequence
    (:then_0
      (if (Utilities|Enum|NotEqual(Enum) Conflicted%20 "NewEnumerator5")
        (bind _returnvalue (Game|ConstructObjectfromClass "/Game/QualityMenu/Blueprints/Util/Keybinding/BP_KeyConflict.BP_KeyConflict_C" self Conflicted%20Combination Conflicted%20))
        (Utilities|Array|Add (Variables|Default|GetConflicting%20Mappings%20Info) _returnvalue) ; Add list of potential conflicts\nso menu can display them.
      ))
    (:then_1
      (if (|SelectBlockingInputTypes Conflicted%20)
        (bind _returnvalue_2 (Game|ConstructObjectfromClass "/Game/QualityMenu/Blueprints/Util/Keybinding/BP_KeyConflict.BP_KeyConflict_C" self Conflicted%20Combination Conflicted%20))
        (Utilities|Array|Add (Variables|Default|GetConflicting%20Mappings%20Blocked) _returnvalue_2) ; Add to list of conflicts that will\nblock input during gameplay
      ))))

(fn ClearConflictingCombinations
  (Utilities|Array|Clear (Variables|Default|GetConflicting%20Mappings%20Info))
  (Utilities|Array|Clear (Variables|Default|GetConflicting%20Mappings%20Blocked)))

(fn EvaluateBlockingCombinations
  (params (Player%20Controller :type Player%20Controller%20Object%20Reference))
  (bind _conflicts_active (LocalVariables|GetConflicts%20Active))
  (bind _returnvalue (> _conflicts_active 0))
  (for _array_element (Variables|Default|GetConflicting%20Mappings%20Blocked) ; Iterate list of blocking conflicts\nand see if one or more is active
    (bind (_axis_value _is_active _just_pressed _just_released) (CallFunction|KeyCombinationCurrentState (Variables|/Game/QualityMenu/Blueprints/Util/Keybinding/BP_KeyConflict.BP_KeyConflict_C|GetConflicting%20Combination _array_element) Player%20Controller true))
    (Utilities|IncrementIntifTrue (LocalVariables|GetConflicts%20Active) _is_active
      (:%20%20
        (Utilities|IncrementIntifTrue (LocalVariables|GetConflicts%20Just%20Pressed) _just_pressed
          (:%20%20
            (Utilities|IncrementIntifTrue (LocalVariables|GetConflicts%20Just%20Released) _just_released))))))
  (return _returnvalue (and _returnvalue (== (LocalVariables|GetConflicts%20Active) (LocalVariables|GetConflicts%20Just%20Pressed))) (and (== (LocalVariables|GetConflicts%20Active) 0) (> (LocalVariables|GetConflicts%20Just%20Released) 0))))

(fn EqualAllConflicts
  (params (Conflicts :type Array%20of%20S%20Key%20Conflict%20Structures))
  (bind _returnvalue (Utilities|Array|Length Conflicts))
  (for _array_element Conflicts ; Compare new array list of conflicts is equal to current one
    (for _array_element_2 (Variables|Default|GetConflicting%20Mappings%20Info)
      (Utilities|IncrementIntifTrue (LocalVariables|GetMatching%20Conflicts) (and (== (Variables|/Game/QualityMenu/Blueprints/Util/Keybinding/BP_KeyConflict.BP_KeyConflict_C|GetConflicting%20Combination _array_element_2) (.conflictingcombination _array_element)) (Utilities|Enum|Equal(Enum) (Variables|/Game/QualityMenu/Blueprints/Util/Keybinding/BP_KeyConflict.BP_KeyConflict_C|GetConflict%20Type _array_element_2) (.conflicttype _array_element))))))
  (return (and (== (Utilities|Array|Length (Variables|Default|GetConflicting%20Mappings%20Info)) _returnvalue) (== _returnvalue (LocalVariables|GetMatching%20Conflicts)))))

(fn EqualAllKeys
  (params (Combination :type Array%20of%20S%20Key%20Input%20Structures))
  (bind _key_inputs (Variables|Default|GetKey%20Inputs))
  (bind _returnvalue (Utilities|Array|Length _key_inputs))
  (for _array_element Combination
    (for _array_element_2 (Variables|Default|GetKey%20Inputs)
      (Utilities|IncrementIntifTrue (LocalVariables|GetMatching%20Keys) (and (== (Variables|/Game/QualityMenu/Blueprints/Util/Keybinding/BP_KeyInput.BP_KeyInput_C|GetKey%20Input _array_element_2) (.input _array_element)) (Math|Boolean|Equal(Boolean) (Variables|/Game/QualityMenu/Blueprints/Util/Keybinding/BP_KeyInput.BP_KeyInput_C|GetAnalog%20Use%20Negative%20Axis _array_element_2) (.usenegativeaxis _array_element))))))
  (return (and (== (Utilities|Array|Length Combination) _returnvalue) (== _returnvalue (LocalVariables|GetMatching%20Keys)))))

(fn AddKeyInput
  (params (InputPin :type S%20Key%20Input%20Structure))
  (bind _input (Utilities|Struct|BreakSKeyInput InputPin))
  (bind _self self)
  (if (or (== _input "AnyKey") (Utilities|Enum|Equal(Enum) (Class|KismetInputLibrary|KeyGetDisplayName _input) (Utilities|Text|MakeLiteralText "None"))) ; Ignore Any Key or None
    (return 0)
    (else
      (bind _returnvalue (Utilities|ReplaceKeyMapping InputPin)) ; Get analog axis representation of some inputs
      (if (Class|KismetInputLibrary|KeyIsFloatAxis (.input _returnvalue)) ; Is key float axis
        (if (or (== (.input _returnvalue) "MouseX") (== (.input _returnvalue) "MouseY")) ; Is key mouse movement
          ;[1 1 1] Store keys in child blueprints, (A small speed improvement)
          (bind _returnvalue_2 (Game|ConstructObjectfromClass "/Game/QualityMenu/Blueprints/Util/Keybinding/BP_KeyInput_AnalogAxis_RemoveDelta.BP_KeyInput_AnalogAxis_RemoveDelta_C" _self))
          (LocalVariables|SetKeyType _returnvalue_2)
          (else
            (bind _returnvalue_3 (Game|ConstructObjectfromClass "/Game/QualityMenu/Blueprints/Util/Keybinding/BP_KeyInput_AnalogAxis.BP_KeyInput_AnalogAxis_C" _self))
            (LocalVariables|SetKeyType _returnvalue_3)))
        (else
          (bind _returnvalue_4 (Game|ConstructObjectfromClass "/Game/QualityMenu/Blueprints/Util/Keybinding/BP_KeyInput_Digital.BP_KeyInput_Digital_C" _self))
          (LocalVariables|SetKeyType _returnvalue_4)))
      (bind _input_2 (Default|InitKeyInput (LocalVariables|GetKeyType) InputPin))
      (Utilities|Array|Add (Variables|Default|GetKey%20Inputs) _input_2)
      (return _input_2))))

(fn GetKeyCombinationDisplayName
  (params (Separator :type String) (No%20Key%20Display :type String) (Display%20Type :type EKeyCombinationDisplay%20Enum))
  (if (> (Utilities|Array|Length (Variables|Default|GetKey%20Inputs)) 0)
    (for (_array_element _array_index) (Variables|Default|GetKey%20Inputs) ; Iterate individual keys that\nmake up key combination
      (Utilities|FlowControl|Sequence
        (:then_0
          (if (> _array_index 0)
            (LocalVariables|SetMapping%20Text (Utilities|String|Append (LocalVariables|GetMapping%20Text) Separator)) ; Only add seperator if\nmore then one key input
          ))
        (:then_1
          (switch Utilities|FlowControl|Switch|SwitchonEKeyCombinationDisplay Display%20Type
            (:NewEnumerator0
              (LocalVariables|SetMapping%20Text (Utilities|String|Append (LocalVariables|GetMapping%20Text) (|GenerateShortUnicode (Variables|/Game/QualityMenu/Blueprints/Util/Keybinding/BP_KeyInput.BP_KeyInput_C|GetDisplay%20Name _array_element)))))
            (:NewEnumerator1
              (LocalVariables|SetMapping%20Text (Utilities|String|Append (LocalVariables|GetMapping%20Text) (|GenerateShortAscii (Variables|/Game/QualityMenu/Blueprints/Util/Keybinding/BP_KeyInput.BP_KeyInput_C|GetDisplay%20Name _array_element)))))
            (:NewEnumerator2
              (LocalVariables|SetMapping%20Text (Variables|/Game/QualityMenu/Blueprints/Util/Keybinding/BP_KeyInput.BP_KeyInput_C|GetDisplay%20Name _array_element)) ; Raw is the unmodified key display
            )))))
    (return (LocalVariables|GetMapping%20Text))
    (else
      (return No%20Key%20Display))))